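; Road decal template, a dismantlable actor with four line helper components that appear in game while a character targets it for dismantling.
; At BeginPlay, RemoveHelpers flags helpers that are invisible or already flagged and disables their collision, then all helpers are hidden.
; Dismantle look start and stop events toggle ShowHideHelpers, which keeps flagged helpers hidden, though LineHelper3 and LineHelper4 check RemoveHelper1 instead of their own flags.
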(event EventBeginPlay
  (CallFunction|RemoveHelpers)
  (CallFunction|ShowHideHelpers false)
  (|CallParentFunction))

(event EventStartIsLookedatforDismantle
  (params (byCharacter :type FG%20Character%20Player%20Object%20Reference))
  (CallFunction|ShowHideHelpers true)
  (|CallParentFunction byCharacter))

(event EventStopIsLookedatforDismantle
  (params (byCharacter :type FG%20Character%20Player%20Object%20Reference))
  (CallFunction|ShowHideHelpers false)
  (|CallParentFunction byCharacter))

(fn ConstructionScript)

(fn ShowHideHelpers
  (params (ShowHelpers :type Boolean))
  (Development|SetHiddeninGame (Variables|Default|GetLineHelper1) (or (Variables|Default|GetRemoveHelper1) (not ShowHelpers)) false)
  (Development|SetHiddeninGame (Variables|Default|GetLineHelper2) (or (Variables|Default|GetRemoveHelper2) (not ShowHelpers)) false)
  (Development|SetHiddeninGame (Variables|Default|GetLineHelper3) (or (Variables|Default|GetRemoveHelper1) (not ShowHelpers)) false)
  (Development|SetHiddeninGame (Variables|Default|GetLineHelper4) (or (Variables|Default|GetRemoveHelper1) (not ShowHelpers)) false))

(fn RemoveHelpers
  (bind _output_get (Variables|Default|SetRemoveHelper1 (or (not (Rendering|IsVisible (Variables|Default|GetLineHelper1))) (Variables|Default|GetRemoveHelper1))))
  (if _output_get
    (Collision|SetCollisionEnabled (Variables|Default|GetLineHelper1) "NoCollision"))
  (bind _output_get_2 (Variables|Default|SetRemoveHelper2 (or (not (Rendering|IsVisible (Variables|Default|GetLineHelper2))) (Variables|Default|GetRemoveHelper2))))
  (if _output_get_2
    (Collision|SetCollisionEnabled (Variables|Default|GetLineHelper2) "NoCollision"))
  (bind _output_get_3 (Variables|Default|SetRemoveHelper3 (or (not (Rendering|IsVisible (Variables|Default|GetLineHelper3))) (Variables|Default|GetRemoveHelper3))))
  (if _output_get_3
    (Collision|SetCollisionEnabled (Variables|Default|GetLineHelper3) "NoCollision"))
  (bind _output_get_4 (Variables|Default|SetRemoveHelper4 (or (not (Rendering|IsVisible (Variables|Default|GetLineHelper4))) (Variables|Default|GetRemoveHelper4))))
  (if _output_get_4
    (Collision|SetCollisionEnabled (Variables|Default|GetLineHelper4) "NoCollision")))